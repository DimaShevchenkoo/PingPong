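; AI-controlled paddle pawn that tracks the moving ball along the Y axis, as in a Pong-style game.
; Each Tick it clamps its Y position within fixed symmetric limits, then looks up BP_MovingBall with GetActorOfClass.
; It applies full movement input toward the ball's Y side, with no dead zone or reaction delay.
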(event `self.ReceiveTick`
  (params (DeltaSeconds :type "Float (single-precision)"))
  (bind (_returnvalue_x _returnvalue_y _returnvalue_z) (`KismetMathLibrary.BreakVector` (`self.K2_GetActorLocation`)))
  (bind (_returnvalue_x_2 _returnvalue_y_2) (`KismetMathLibrary.BreakVector` (`self.K2_GetActorLocation`)))
  (if (> _returnvalue_y 565.0)
    (`self.K2_SetActorLocation` (`KismetMathLibrary.MakeVector` _returnvalue_x 565.0 _returnvalue_z))
    (elif (< _returnvalue_y -565.0)
      (`self.K2_SetActorLocation` (`KismetMathLibrary.MakeVector` _returnvalue_x -565.0 _returnvalue_z))))
  (bind _returnvalue (`GameplayStatics.GetActorOfClass` "/Game/BluePrints/Actors/BP_MovingBall.BP_MovingBall_C"))
  (bind (_returnvalue_x_3 _returnvalue_y_3) (`KismetMathLibrary.BreakVector` (`self.K2_GetActorLocation` _returnvalue)))
  (`self.AddMovementInput` (`KismetMathLibrary.MakeVector` 0.0 (select `bool` (> (- _returnvalue_y_3 _returnvalue_y_2) 0.0) :`false` -1.0 :`true` 1.0 :!type "Float (single-precision)"))))

(fn `UserConstructionScript`
  (`parent.UserConstructionScript`))